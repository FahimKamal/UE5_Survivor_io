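; BP_Pickup_master is a pickup actor for coins and health that spins on a looping timeline.
; On first sphere overlap with BP_Player, a DoOnce-gated timeline flies it to the player's current position while shrinking it to zero.
; A switch on PickupType then grants the reward: Coin adds BaseValue experience, plays a sound and destroys the actor.
; Health only calls AddPlayerHealth, without sound or destruction.
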(event `self.ReceiveBeginPlay`
  (set `self.StartingPickupLocation` (`self.K2_GetActorLocation`))
  (`self.Spin Coin`))

(event `Spin Coin`
  ;[0.5824 0.6171 0.7281] Spin the coin in the scene.
  (bind (_direction _timer) (`Timeline|Timeline` :!via `PlayFromStart` :!label _label)
    (:`Update`
      (`self.K2_SetActorRotation` (`KismetMathLibrary.MakeRotator` 0.0 0.0 (`KismetMathLibrary.Lerp` 0.0 360.0 _timer))))
    (:`Finished`
      (goto _label :!via `PlayFromStart`))))

(event `self.Sphere.OnComponentBeginOverlap`
  (params (OverlappedComponent :type "PrimitiveComponent Object Reference") (OtherActor :type "Actor Object Reference") (OtherComp :type "PrimitiveComponent Object Reference") (OtherBodyIndex :type Integer) (bFromSweep :type Boolean) (SweepResult :type "HitResult Structure (by ref)"))
  ;[0.5824 0.6171 0.7281] Coin overlap with player functionality.
  (`/Engine/EditorBlueprintResources/StandardMacros.DoOnce` false :!label _label_2
    (:`Completed`
      (bind _asbp_player (cast `/Game/Blueprint/Player/BP_Player` OtherActor)
        (:`then`
          (set `self.As BP Player` _asbp_player)
          (bind (_direction _alpha) (`Timeline|ShrinkCoinAndGoToPlayer` :!via `PlayFromStart`)
            (:`Update`
              (`self.K2_SetActorLocation` (`KismetMathLibrary.VLerp` (`self.StartingPickupLocation`) (`self.K2_GetActorLocation` (`self.As BP Player`)) _alpha))
              (`self.SetActorScale3D` (`KismetMathLibrary.VLerp` (0.3 0.3 0.3) (0.0 0.0 0.0) _alpha)))
            (:`Finished`
              (switch `/Game/Blueprint/Pickups/E_PickupType` (`self.Pickup Type`)
                (:`NewEnumerator0`
                  (`/Game/Blueprint/Player/BP_Player.Add Coin Experience` (`self.As BP Player`) (`self.BaseValue`))
                  (`GameplayStatics.PlaySoundAtLocation` "/Game/Assets/Sounds/coins/Coin.Coin" (`self.K2_GetActorLocation`) (struct) 1.0 1.0 0.0 null null null null)
                  (`self.K2_DestroyActor`))
                (:`NewEnumerator1`
                  (`/Game/Blueprint/Player/BP_Player.Add Player Health` (`self.As BP Player`)))))))
        (:`CastFailed`
          (goto _label_2 :!via `Reset`))))))

(fn `UserConstructionScript`)