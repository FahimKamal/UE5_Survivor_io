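; Master Blueprint for slime enemies that chase the player, deal contact damage and take damage from spells.
; AI MoveTo repeats after each successful arrival, and a sphere overlap hurts the player through a delay-reset DoOnce cooldown.
; Spell hits apply slightly randomized damage, updating the health bar widget, playing sound and damage numbers, and flashing a dynamic material via timeline.
; On death it drops a coin pickup matching the slime type.
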(event `self.ReceiveBeginPlay`
  ;[0.5824 0.6171 0.7281] Get ref of the enemy health bar
  (bind _aswbp_enemy_health (cast `/Game/Blueprint/Enemies/WBP_EnemyHealth` (`WidgetComponent.GetWidget` (`self.HealthBar`))))
  (set `self.EnemyHealthBar` _aswbp_enemy_health)
  ;[0.5824 0.6171 0.7281] Move enemy towards player
  (`|AIMoveTo` self (0.0 0.0 0.0) (`GameplayStatics.GetPlayerCharacter` 0) 50.0 :!label _label
    (:`OnSuccess`
      (`KismetSystemLibrary.Delay` 0.8)
      (goto _label))))

(event `self.Sphere.OnComponentBeginOverlap`
  (params (OverlappedComponent :type "PrimitiveComponent Object Reference") (OtherActor :type "Actor Object Reference") (OtherComp :type "PrimitiveComponent Object Reference") (OtherBodyIndex :type Integer) (bFromSweep :type Boolean) (SweepResult :type "HitResult Structure (by ref)"))
  ;[0.5824 0.6171 0.7281] If Collide with player deal damage.
  (bind _asbp_player (cast `/Game/Blueprint/Player/BP_Player` OtherActor))
  (`/Engine/EditorBlueprintResources/StandardMacros.DoOnce` false :!label _label_2
    (:`Completed`
      (`/Game/Blueprint/Player/BP_Player.Get Hurt and Update Health` _asbp_player (`self.Enemy Damage`))
      (`KismetSystemLibrary.Delay` 0.8)
      (goto _label_2 :!via `Reset`))))

(event `/Game/Blueprint/Enemies/BPI_Enemies.SpellCollisionEvent`
  (params (SpellDamageInput :type "Float (double-precision)"))
  (bind _returnvalue (`self.GetTransform`))
  (bind _returnvalue_2 (- (`self.EnemyCurrentHealth`) (+ SpellDamageInput (`KismetMathLibrary.RandomFloatInRange` -5.0 5.0))))
  ;[0.5824 0.6171 0.7281] Damage system by player spells
  (bind _output_get (set `self.EnemyCurrentHealth` (`KismetMathLibrary.FClamp` _returnvalue_2 0.0 (`self.EnemyMaxHealth`))))
  (if (> _output_get 0.0)
    (`self.UpdateHealthUI` _output_get)
    (`GameplayStatics.PlaySoundAtLocation` "/Game/Assets/Sounds/ImpactSlime/SlimeImpact.SlimeImpact" (`self.K2_GetActorLocation`) (struct) 1.0 1.0 0.0 null null null null)
    (`self.EnemyFlashingEffect`)
    (`/Game/Blueprint/Enemies/WBP_EnemyHealth.PlayDamageNumberAnimation` (`self.EnemyHealthBar`) _returnvalue_2)
    (else
      (switch `/Game/Blueprint/Enemies/E_SlimeType` (`self.SlimeType`)
        (:`NewEnumerator0`
          (`|SpawnActorFromClass` "/Game/Blueprint/Pickups/BP_Pickup_Copper.BP_Pickup_Copper_C" _returnvalue "Undefined" "MultiplyWithRoot" null null))
        (:`NewEnumerator1`
          (`|SpawnActorFromClass` "/Game/Blueprint/Pickups/BP_Pickup_Silver.BP_Pickup_Silver_C" _returnvalue "Undefined" "MultiplyWithRoot" null null))
        (:`NewEnumerator2`
          (`|SpawnActorFromClass` "/Game/Blueprint/Pickups/BP_Pickup_Gold.BP_Pickup_Gold_C" _returnvalue "Undefined" "MultiplyWithRoot" null null)))
      (`self.K2_DestroyActor`))))

(event `EnemyFlashingEffect`
  ;[1 1 1] Flashing effect on getting hit
  (bind (_direction _flashalpha) (`Timeline|FlashingTimer` :!via `PlayFromStart`)
    (:`Update`
      (`MaterialInstanceDynamic.SetScalarParameterValue` (`self.Ref Material`) "Emissive" _flashalpha))))

(fn `UpdateHealthUI`
  (params (HealthPercentage :type "Float (double-precision)"))
  (`/Game/Blueprint/Enemies/WBP_EnemyHealth.UpdatePercentage` (`self.EnemyHealthBar`) (/ HealthPercentage (`self.EnemyMaxHealth`))))

(fn `UserConstructionScript`
  (bind _returnvalue (`KismetMaterialLibrary.CreateDynamicMaterialInstance` (`self.SlimeMat_ref`)))
  (bind _output_get (set `self.Ref Material` _returnvalue))
  (`PrimitiveComponent.SetMaterial` (`self.Mesh_Slime`) 0 _output_get))