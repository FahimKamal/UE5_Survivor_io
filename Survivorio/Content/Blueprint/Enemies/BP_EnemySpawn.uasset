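; Enemy spawner that periodically creates four tiers of slimes (poison, mud, dark and king) around the edges of a square area.
; BeginPlay starts a looping poison slime timer, while separate events start the timers for the higher tiers.
; Tier events feed name and stats into FSpawnSlimes, which picks a random edge and point, then spawns the matching slime class with that health and damage.
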(event `self.ReceiveBeginPlay`
  (`KismetSystemLibrary.K2_SetTimerDelegate` (`|CreateDelegate` :!event `Spawn Poison Slimes`) (`self.Spawn Timer Poison Slime`) true))

(event `Spawn Poison Slimes`
  (`self.F Spawn Slimes` "Level1"))

(event `Spawn Mud Slimes`
  (`self.F Spawn Slimes` "Level2" 100.0 100.0 15.0))

(event `Spawn Dark Slimes`
  (`self.F Spawn Slimes` "Level3" 300.0 300.0 20.0))

(event `Start Timer Mud Slimes`
  (`KismetSystemLibrary.K2_SetTimerDelegate` (`|CreateDelegate` :!event `Spawn Mud Slimes`) (`self.Spawn Timer Mud Slime`) true))

(event `Spawn King Slimes`
  (`self.F Spawn Slimes` "Level4" 700.0 700.0 20.0))

(event `Start Timer Dark Slimes`
  (`KismetSystemLibrary.K2_SetTimerDelegate` (`|CreateDelegate` :!event `Spawn Dark Slimes`) (`self.Spawn Timer Dark Slime`) true))

(event `Start Timer King Slimes`
  (`KismetSystemLibrary.K2_SetTimerDelegate` (`|CreateDelegate` :!event `Spawn King Slimes`) (`self.Spawn Timer King Slime`) true))

(fn `F Spawn Slimes`
  (params (`Enemy Name` :type String) (`Enemy Max Health` :type "Float (double-precision)" :default 50.0) (`Enemy Current Health` :type "Float (double-precision)" :default 50.0) (`Enemy Damage` :type "Float (double-precision)" :default 10.0))
  (locals (`Max Health` :type "Float (double-precision)") (`Current Health` :type "Float (double-precision)") (Damage :type "Float (double-precision)"))
  (set `local.Max Health` `Enemy Max Health`)
  (set `local.Current Health` `Enemy Current Health`)
  (set `local.Damage` `Enemy Damage`)
  ;[1 1 1] Select a random location between a range and spawn enemy at the edge.
  (switch `int` (`KismetMathLibrary.RandomIntegerInRange` 1 4)
    (:`1`
      (set `self.Location` (`KismetMathLibrary.MakeVector` (`KismetMathLibrary.RandomFloatInRange` -2400.0 2400.0) 2400.0 220.0)))
    (:`2`
      (set `self.Location` (`KismetMathLibrary.MakeVector` (`KismetMathLibrary.RandomFloatInRange` -2400.0 2400.0) -2400.0 220.0)))
    (:`3`
      (set `self.Location` (`KismetMathLibrary.MakeVector` 2400.0 (`KismetMathLibrary.RandomFloatInRange` -2400.0 2400.0) 220.0)))
    (:`4`
      (set `self.Location` (`KismetMathLibrary.MakeVector` -2400.0 (`KismetMathLibrary.RandomFloatInRange` -2400.0 2400.0) 220.0))))
  (switch `string` `Enemy Name`
    (:`Level1`
      (`|SpawnActorFromClass` "/Game/Blueprint/Enemies/BP_SlimePoison.BP_SlimePoison_C" (`KismetMathLibrary.MakeTransform` (`self.Location`)) "Undefined" "MultiplyWithRoot" null (`local.Damage`) (`local.Max Health`) (`local.Current Health`) null))
    (:`Level2`
      (`|SpawnActorFromClass` "/Game/Blueprint/Enemies/BP_SlimeMud.BP_SlimeMud_C" (`KismetMathLibrary.MakeTransform` (`self.Location`)) "Undefined" "MultiplyWithRoot" null (`local.Damage`) (`local.Max Health`) (`local.Current Health`) null))
    (:`Level3`
      (`|SpawnActorFromClass` "/Game/Blueprint/Enemies/BP_SlimeDark.BP_SlimeDark_C" (`KismetMathLibrary.MakeTransform` (`self.Location`)) "Undefined" "MultiplyWithRoot" null (`local.Damage`) (`local.Max Health`) (`local.Current Health`) null))
    (:`Level4`
      (`|SpawnActorFromClass` "/Game/Blueprint/Enemies/BP_SlimeBoss.BP_SlimeBoss_C" (`KismetMathLibrary.MakeTransform` (`self.Location`)) "Undefined" "MultiplyWithRoot" null (`local.Damage`) (`local.Max Health`) (`local.Current Health`) null))))

(fn `UserConstructionScript`)