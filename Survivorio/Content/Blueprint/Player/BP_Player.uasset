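; Player character for a top-down, survivors-style game: it moves by input, faces the cursor, casts spells, gains XP and takes damage.
; Leveled fire, ice, orbiting earth and wind spells spawn projectile actors from rotating pivots.
; BeginPlay creates the HUD and enemy spawner; a minute counter escalates slime spawns until victory at minute eight.
; Level-ups pause for skill selection, and zero health shows the death screen.
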(event `InitializeEarthSpell`
  (params (`Number of Orbs` :type Integer) (`Orb Rotation` :type "Float (double-precision)"))
  (bind _orbspell_spawn (`self.OrbSpell Spawn`))
  ;[0.6933 0.147 1] Orb Spell
  ;;[0.3186 1 0.3008] Initialize Earth spell
  (for _ (range 1 (+ `Number of Orbs` 1))
    (bind _returnvalue (`|SpawnActorFromClass` "/Game/Blueprint/Player/Spells/BP_Spell_Orb.BP_Spell_Orb_C" (`KismetMathLibrary.MakeTransform` (`SceneComponent.K2_GetComponentLocation` _orbspell_spawn) (`SceneComponent.K2_GetComponentRotation` _orbspell_spawn)) "Undefined" "MultiplyWithRoot" null null))
    (`self.K2_AttachToComponent` _returnvalue (`self.Orb Rotating Pivot`) "None" "KeepWorld" "KeepWorld" "KeepWorld" true)
    (`SceneComponent.K2_AddLocalRotation` (`self.OrbSpell Pivot`) (`KismetMathLibrary.MakeRotator` 0.0 0.0 `Orb Rotation`) false false)))

(event `Start FireBall`
  ;[1 0.4434 0.09368] Fire Ball
  (switch `int` (`self.SpellLevel_Fire`)
    (:`1`
      (`self.SpellSpawnFireballs` 1))
    (:`2`
      (`self.SpellSpawnFireballs` 2 -10.0 20.0))
    (:`3`
      (`self.SpellSpawnFireballs` 3 -15.0 15.0))
    (:`4`
      (`self.SpellSpawnFireballs` 4 -15.0 10.0))
    (:`5`
      (`self.SpellSpawnFireballs` 5 -20.0 10.0))))

(event `Start Rotating Earth`
  ;[0.6933 0.147 1] Orb Spell
  ;;[0.3186 1 0.3008] Rorate the earth orbs after spawning them.
  (bind (_direction _newtrack_0) (`Timeline|Timeline` :!via `PlayFromStart`)
    (:`Update`
      (`SceneComponent.K2_SetRelativeRotation` (`self.Orb Rotating Pivot`) (`KismetMathLibrary.MakeRotator` 0.0 0.0 (`KismetMathLibrary.Lerp` 0.0 360.0 _newtrack_0)) false false))
    (:`Finished`
      (`self.Start Rotating Earth`))))

(event `Start EarthSpell`
  ;[0.6933 0.147 1] Orb Spell
  ;;[0.3186 1 0.3008] Delete the existing earth orbs and initialize earh spell each time the spell upgrades.
  (bind _outactors (`GameplayStatics.GetAllActorsOfClass` "/Game/Blueprint/Player/Spells/BP_Spell_Orb.BP_Spell_Orb_C"))
  (for _array_element _outactors
    (`self.K2_DestroyActor` _array_element))
  (switch `int` (`self.SpellLevel_Orb`)
    (:`1`
      (`self.InitializeEarthSpell` 3 120.0))
    (:`2`
      (`self.InitializeEarthSpell` 4 90.0))
    (:`3`
      (`self.InitializeEarthSpell` 5 72.0))
    (:`4`
      (`self.InitializeEarthSpell` 6 60.0))
    (:`5`
      (`self.InitializeEarthSpell` 8 45.0))))

(event `Start Ice Spell`
  ;[0.1256 0.8255 1] Ice Spell
  (`KismetSystemLibrary.K2_SetTimerDelegate` (delegate `Ice Spell`) 1.5 true))

(event `Ice Spell`
  ;[0.1256 0.8255 1] Ice Spell
  (switch `int` (`self.SpellLevel_Ice`)
    (:`1`
      (`self.SpellSpawnIceBalls` 3 120.0))
    (:`2`
      (`self.SpellSpawnIceBalls` 4 90.0))
    (:`3`
      (`self.SpellSpawnIceBalls` 5 72.0))
    (:`4`
      (`self.SpellSpawnIceBalls` 6 60.0))
    (:`5`
      (`self.SpellSpawnIceBalls` 8 45.0))))

(event `InitializeWindSpell`
  (bind _windspell_pivot (`self.WindSpell Pivot`))
  ;[0.3186 1 0.3008] Wind Spell
  ;;[1 1 1] Initialize Wind Spell
  (`SceneComponent.K2_SetRelativeRotation` _windspell_pivot (`KismetMathLibrary.MakeRotator` 0.0 0.0 (`KismetMathLibrary.RandomFloatInRange` 0.0 360.0)) false false)
  (`|SpawnActorFromClass` "/Game/Blueprint/Player/Spells/BP_Spell_Wind.BP_Spell_Wind_C" (`KismetMathLibrary.MakeTransform` (`SceneComponent.K2_GetComponentLocation` _windspell_pivot) (`SceneComponent.K2_GetComponentRotation` _windspell_pivot)) "Undefined" "MultiplyWithRoot" null null))

(event `Start Wind Spell`
  ;[0.3186 1 0.3008] Wind Spell
  ;;[1 1 1] Start Wind Spell
  (switch `int` (`self.SpellLevel_Wind`)
    (:`1`
      (set `self.WindSpawnSpeed` 2.0)
      (`self.InitializeWindSpell`))
    (:`2`
      (set `self.WindSpawnSpeed` 1.6)
      (`self.InitializeWindSpell`))
    (:`3`
      (set `self.WindSpawnSpeed` 1.2)
      (`self.InitializeWindSpell`))
    (:`4`
      (set `self.WindSpawnSpeed` 0.8)
      (`self.InitializeWindSpell`))
    (:`5`
      (set `self.WindSpawnSpeed` 0.01)
      (`self.InitializeWindSpell`))))

(event `self.ReceiveBeginPlay`
  ;[0.5824 0.6171 0.7281] Create Widget, set ref and add to viewport
  (bind _returnvalue (`|CreateWidget` "/Game/Blueprint/Player/Widgets/WBP_Player.WBP_Player_C"))
  (bind _output_get (set `self.Ref_Widget` _returnvalue))
  (`UserWidget.AddToViewport` _output_get 0)
  (`KismetSystemLibrary.K2_SetTimerDelegate` (`|CreateDelegate` :!event `Start FireBall`) 1.0 true)
  (bind _returnvalue_2 (`|SpawnActorFromClass` "/Game/Blueprint/Enemies/BP_EnemySpawn.BP_EnemySpawn_C" (`self.GetTransform`) "Undefined" "MultiplyWithRoot" null null))
  (set `self.Ref Spawner` _returnvalue_2)
  (`KismetSystemLibrary.K2_SetTimerDelegate` (`|CreateDelegate` :!event `Update Timer`) 1.0 true))

(event `Start Wind Spell Timer`
  ;[0.3186 1 0.3008] Wind Spell
  ;;[1 1 1] Wind Spell Loop timer
  (`KismetSystemLibrary.K2_SetTimerDelegate` (`|CreateDelegate` :!event `Start Wind Spell`) (`self.WindSpawnSpeed`) true))

(event `EnhancedInput|/Game/Blueprint/Player/IA_Movement`
  (params (ActionValue :type "Vector2D Structure") (ElapsedSeconds :type "Float (double-precision)") (TriggeredSeconds :type "Float (double-precision)") (InputAction :type "InputAction Object Reference" :default "/Game/Blueprint/Player/IA_Movement.IA_Movement"))
  ;[0.5824 0.6171 0.7281] Movement of the player
  (:`Triggered`
    (`self.AddMovementInput` (1.0 0.0 0.0) ActionValue_X)
    (`self.AddMovementInput` (0.0 1.0 0.0) ActionValue_Y)))

(event `Update Timer`
  ;[1 1 1] Timer logic call every 1 second
  (bind _result (`/Engine/EditorBlueprintResources/StandardMacros.IncrementInt` (`self.Seconds`))
    (:`  `
      (if (== _result 60)
        (set `self.Seconds` 0)
        (bind _result_2 (`/Engine/EditorBlueprintResources/StandardMacros.IncrementInt` (`self.Minutes`))
          (:`  `
            (`self.Update Level Difficulty`))))
      (`/Game/Blueprint/Player/Widgets/WBP_Player.Update Timer` (`self.Ref_Widget`) _result_2 (`self.Seconds`)))))

(event `Update Level Difficulty`
  (bind _ref_spawner (`self.Ref Spawner`))
  (switch `int` (`self.Minutes`)
    (:`1`
      (set `/Game/Blueprint/Enemies/BP_EnemySpawn.Spawn Timer Poison Slime` 0.8 _ref_spawner))
    (:`2`
      (`/Game/Blueprint/Enemies/BP_EnemySpawn.Start Timer Mud Slimes` _ref_spawner))
    (:`3`
      (set `/Game/Blueprint/Enemies/BP_EnemySpawn.Spawn Timer Mud Slime` 0.8 _ref_spawner))
    (:`4`
      (`/Game/Blueprint/Enemies/BP_EnemySpawn.Start Timer Dark Slimes` _ref_spawner))
    (:`5`
      (set `/Game/Blueprint/Enemies/BP_EnemySpawn.Spawn Timer Dark Slime` 1.0 _ref_spawner))
    (:`6`
      (`/Game/Blueprint/Enemies/BP_EnemySpawn.Start Timer King Slimes` _ref_spawner))
    (:`7`
      (set `/Game/Blueprint/Enemies/BP_EnemySpawn.Spawn Timer King Slime` 1.0 _ref_spawner))
    (:`8`
      (`self.Player Wins`))))

(event `Add Coin Experience`
  (params (`Pickup Value` :type "Float (double-precision)"))
  ;[0.5824 0.6171 0.7281] Add experiment points for collecting coins
  (set `self.CurrentExperience` (+ (`self.CurrentExperience`) `Pickup Value`))
  (`/Game/Blueprint/Player/Widgets/WBP_Player.UpdateXP_Percentage` (`self.Ref_Widget`) (/ (`self.CurrentExperience`) (`self.ExperienceCap`)))
  ;[1 1 1] Level up character and give option to select new and upgrade skills
  (if (>= (`self.CurrentExperience`) (`self.ExperienceCap`))
    (`/Game/Blueprint/Player/Widgets/WBP_Player.UpdateXP_Percentage` (`self.Ref_Widget`) 0.0)
    (`/Engine/EditorBlueprintResources/StandardMacros.IncrementInt` (`self.CharacterLevel`)
      (:`  `
        (set `self.CurrentExperience` 0.0)
        (`/Game/Blueprint/Player/Widgets/WBP_Player.Increase Player Level` (`self.Ref_Widget`) (`self.CharacterLevel`))
        (if (< (`self.CharacterLevel`) 20)
          (`self.Start Selecting Skills`))))))

(event `Player Wins`
  (bind _returnvalue (`GameplayStatics.GetPlayerController` 0))
  (`GameplayStatics.SetGamePaused` true)
  (`WidgetBlueprintLibrary.SetInputMode_UIOnlyEx` _returnvalue null)
  (set `PlayerController.bShowMouseCursor` true _returnvalue)
  (`Widget.SetVisibility` (`/Game/Blueprint/Player/Widgets/WBP_Player.WBP_WinScreen` (`self.Ref_Widget`)) "Visible"))

(event `Get Hurt and Update Health`
  (params (`Enemy Damage` :type "Float (double-precision)"))
  (bind _returnvalue (`GameplayStatics.GetPlayerController` 0))
  (bind _wbp_deathscreen (`/Game/Blueprint/Player/Widgets/WBP_Player.WBP_DeathScreen` (`self.Ref_Widget`)))
  ;[1 1 1] Player get hurt function and update UI
  (bind _output_get (set `self.Player_Health` (`KismetMathLibrary.FClamp` (- (`self.Player_Health`) `Enemy Damage`) 0.0 (`self.Player_MaxHealth`))))
  (`/Game/Blueprint/Player/Widgets/WBP_Player.UpdatePercentage` (`self.Ref_Widget`) (/ _output_get (`self.Player_MaxHealth`)))
  ;[1 1 1] After health reaching zero show death screen.
  (if (<= (`self.Player_Health`) 0.0)
    (`GameplayStatics.SetGamePaused` true)
    (`Widget.SetVisibility` _wbp_deathscreen "Visible")
    (`/Game/Blueprint/Player/Widgets/WBP_DeathScreen.Play Fade Animation` _wbp_deathscreen)
    (`WidgetBlueprintLibrary.SetInputMode_UIOnlyEx` _returnvalue _wbp_deathscreen)
    (set `PlayerController.bShowMouseCursor` true _returnvalue)))

(event `self.ReceiveTick`
  (params (DeltaSeconds :type "Float (single-precision)"))
  (bind (_returnvalue_x _returnvalue_y) (`KismetMathLibrary.BreakVector` (`self.K2_GetActorLocation`)))
  (bind (_bblockinghit _binitialoverlap _time _distance _location) (`GameplayStatics.BreakHitResult` (`PlayerController.GetHitResultUnderCursorByChannel` (`GameplayStatics.GetPlayerController` 0) "TraceTypeQuery1" true)))
  ;[0.5824 0.6171 0.7281] Face player toward the mouse and move crosshair to mouse location.
  (`self.K2_SetActorRotation` (`KismetMathLibrary.FindLookAtRotation` (`KismetMathLibrary.MakeVector` _returnvalue_x _returnvalue_y) (`KismetMathLibrary.MakeVector` (.x _location) (.y _location))))
  (`SceneComponent.K2_SetWorldLocation` (`self.Mesh_Crosshair`) (`KismetMathLibrary.MakeVector` (.x _location) (.y _location)) false false))

(event `Start Selecting Skills`
  (`self.SetUpgradeButtons`)
  (`self.SkillLevelupFunction` true true true))

(event `Return to Game`
  (`self.SkillLevelupFunction` false false false "MOVE_Walking" "Hidden"))

(fn `SkillLevelupFunction`
  (params (bGamePaused :type Boolean) (`bInputModeUI Only` :type Boolean) (`Show Mouse Cursor` :type Boolean) (PlayerMovementMode :type "EMovementMode Enum" :default "MOVE_None") (`UI Visibility` :type "ESlateVisibility Enum" :default "Visible"))
  (bind _returnvalue (`GameplayStatics.GetPlayerController` 0))
  (`GameplayStatics.SetGamePaused` bGamePaused)
  (if `bInputModeUI Only`
    (`WidgetBlueprintLibrary.SetInputMode_UIOnlyEx` _returnvalue (`self.Ref_Widget`))
    (else
      (`WidgetBlueprintLibrary.SetInputMode_GameOnly` _returnvalue)))
  (set `PlayerController.bShowMouseCursor` `Show Mouse Cursor` _returnvalue)
  (`CharacterMovementComponent.SetMovementMode` (`self.CharacterMovement`) PlayerMovementMode 0)
  (`Widget.SetVisibility` (`/Game/Blueprint/Player/Widgets/WBP_Player.WBP_Leveling` (`self.Ref_Widget`)) `UI Visibility`))

(fn `SpellSpawnFireballs`
  (params (`Number of Projectile` :type Integer) (`Start Rotation` :type "Float (double-precision)") (`Rotation Increment` :type "Float (double-precision)"))
  (bind _fireball_spawn (`self.FireBall Spawn`))
  (`SceneComponent.K2_SetRelativeRotation` (`self.FireBall Pivot`) (`KismetMathLibrary.MakeRotator` 0.0 0.0 `Start Rotation`) false false)
  (for _ (range 1 (+ `Number of Projectile` 1))
    (`|SpawnActorFromClass` "/Game/Blueprint/Player/Spells/BP_Spell_Fire.BP_Spell_Fire_C" (`KismetMathLibrary.MakeTransform` (`SceneComponent.K2_GetComponentLocation` _fireball_spawn) (`SceneComponent.K2_GetComponentRotation` _fireball_spawn)) "AdjustIfPossibleButAlwaysSpawn" "MultiplyWithRoot" null null)
    (`SceneComponent.K2_AddRelativeRotation` (`self.FireBall Pivot`) (`KismetMathLibrary.MakeRotator` 0.0 0.0 `Rotation Increment`) false false))
  (`SceneComponent.K2_SetRelativeRotation` :`self` (`self.FireBall Pivot`)))

(fn `SpellSpawnIceBalls`
  (params (`Number of Projectile` :type Integer) (`Rotation Increment` :type "Float (double-precision)"))
  (bind _iceball_spawn (`self.IceBall Spawn`))
  (`SceneComponent.K2_SetRelativeRotation` (`self.IceBall Pivot`) (`KismetMathLibrary.MakeRotator` 0.0 0.0 (`KismetMathLibrary.RandomFloatInRange` 0.0 360.0)) false false)
  (for _ (range 1 (+ `Number of Projectile` 1))
    (`|SpawnActorFromClass` "/Game/Blueprint/Player/Spells/BP_Spell_Ice.BP_Spell_Ice_C" (`KismetMathLibrary.MakeTransform` (`SceneComponent.K2_GetComponentLocation` _iceball_spawn) (`SceneComponent.K2_GetComponentRotation` _iceball_spawn)) "AdjustIfPossibleButAlwaysSpawn" "MultiplyWithRoot" null null)
    (`SceneComponent.K2_AddRelativeRotation` (`self.IceBall Pivot`) (`KismetMathLibrary.MakeRotator` 0.0 0.0 `Rotation Increment`) false false))
  (`SceneComponent.K2_SetRelativeRotation` :`self` (`self.IceBall Pivot`)))

(fn `UserConstructionScript`)