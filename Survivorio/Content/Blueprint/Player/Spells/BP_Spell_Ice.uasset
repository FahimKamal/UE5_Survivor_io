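; BP_Spell_Ice is an ice spell actor that launches from the player as a damaging projectile.
; On spawn it attaches to the player character for a short delay, then plays a whoosh sound, detaches and adds a ProjectileMovement component at runtime to start its flight.
; Its DamageSphere overlap passes SpellDamage to any actor implementing BPI_Enemies through the SpellCollisionEvent interface message.
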(event `self.ReceiveBeginPlay`
  (`self.K2_AttachToActor` (`GameplayStatics.GetPlayerCharacter` 0) "None" "KeepWorld" "KeepWorld" "KeepWorld")
  (`KismetSystemLibrary.Delay` 0.5)
  (`GameplayStatics.PlaySoundAtLocation` "/Game/Assets/Sounds/IceSpell/IceSpellWoosh_Cue.IceSpellWoosh_Cue" (`self.K2_GetActorLocation`) (struct) 1.0 1.0 0.0 null null null null)
  (`self.K2_DetachFromActor` "KeepWorld" "KeepWorld" "KeepWorld")
  (`AddComponent|NODE_AddProjectileMovementComponent-0`))

(event `self.DamageSphere.OnComponentBeginOverlap`
  (params (OverlappedComponent :type "PrimitiveComponent Object Reference") (OtherActor :type "Actor Object Reference") (OtherComp :type "PrimitiveComponent Object Reference") (OtherBodyIndex :type Integer) (bFromSweep :type Boolean) (SweepResult :type "HitResult Structure (by ref)"))
  ;[0.5824 0.6171 0.7281] If collided with enemy deal damage.
  (if (`KismetSystemLibrary.DoesImplementInterface` OtherActor "/Game/Blueprint/Enemies/BPI_Enemies.BPI_Enemies_C")
    (message `/Game/Blueprint/Enemies/BPI_Enemies.SpellCollisionEvent` OtherActor (`self.Spell Damage`))))

(fn `UserConstructionScript`)